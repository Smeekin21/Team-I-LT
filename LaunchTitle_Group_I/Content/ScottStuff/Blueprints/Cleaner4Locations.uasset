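; Moving hazard actor that damages the third-person player character when it overlaps its Box.
; The Construction Script feeds four relative locations and a Duration into an InterpToMovement component to define the path.
; Box overlap applies ScaleDamageAmount as damage, then treats a truncated value of 0, 1 or 2 as a tier and replaces it with a preset amount, affecting only subsequent hits.
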(event `self.Box.OnComponentBeginOverlap`
  (params (OverlappedComponent :type "PrimitiveComponent Object Reference") (OtherActor :type "Actor Object Reference") (OtherComp :type "PrimitiveComponent Object Reference") (OtherBodyIndex :type Integer) (bFromSweep :type Boolean) (SweepResult :type "HitResult Structure (by ref)"))
  (bind _scaledamageamount (`self.ScaleDamageAmount`))
  (bind _asbp_third_person_character (cast `/Game/ThirdPerson/Blueprints/BP_ThirdPersonCharacter` OtherActor))
  (`GameplayStatics.ApplyDamage` _asbp_third_person_character _scaledamageamount)
  (switch `int` (`KismetMathLibrary.FTrunc` _scaledamageamount)
    (:`0`
      (set `self.ScaleDamageAmount` 25.0))
    (:`1`
      (set `self.ScaleDamageAmount` 45.0))
    (:`2`
      (set `self.ScaleDamageAmount` 95.0))))

(event `self.ReceiveBeginPlay`)

(fn `UserConstructionScript`
  (bind _interptomovement (`self.InterpToMovement`))
  ;[1 1 1] Move to 1 point and then pack
  (set `InterpToMovementComponent.ControlPoints` (`|MakeArray` (make `InterpControlPoint` (`self.Location1`)) (make `InterpControlPoint` (`self.Location2`)) (make `InterpControlPoint` (`self.Location3`)) (make `InterpControlPoint` (`self.Location4`))) _interptomovement)
  (set `InterpToMovementComponent.Duration` (`self.Duration`) _interptomovement))