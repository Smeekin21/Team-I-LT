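; Locked sliding double door that opens when a player who has a key presses Interact nearby.
; A box trigger enables the actor's input while a BP_ThirdPersonCharacter overlaps it, caching that character on entry, and disables it on exit.
; Interact checks the cached character's HasKey flag, then plays a timeline that lerps the two door halves between stored relative positions, with no closing logic.
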(event `Key|E`
  (params (Key :type "Key Structure")))

(event `EnhancedInput|/Game/ThirdPerson/Input/Actions/IA_Interact`
  (params (ActionValue :type Boolean) (ElapsedSeconds :type "Float (double-precision)") (TriggeredSeconds :type "Float (double-precision)") (InputAction :type "InputAction Object Reference" :default "/Game/ThirdPerson/Input/Actions/IA_Interact.IA_Interact"))
  (:`Triggered`
    (if (`/Game/ThirdPerson/Blueprints/BP_ThirdPersonCharacter.HasKey?` (stale `self.Box.OnComponentBeginOverlap` _asbp_third_person_character))
      (bind (_direction _slide) (`Timeline|Timeline`)
        (:`Update`
          (`SceneComponent.K2_SetRelativeLocation` (`self.door_huge_top`) (`KismetMathLibrary.VLerp` (`self.CurrentLeft`) (`self.NewLeft`) _slide) false false)
          (`SceneComponent.K2_SetRelativeLocation` (`self.door_huge_bottom`) (`KismetMathLibrary.VLerp` (`self.Current Right`) (`self.NewRight`) _slide) false false))))))

(event `self.Box.OnComponentBeginOverlap`
  (params (OverlappedComponent :type "PrimitiveComponent Object Reference") (OtherActor :type "Actor Object Reference") (OtherComp :type "PrimitiveComponent Object Reference") (OtherBodyIndex :type Integer) (bFromSweep :type Boolean) (SweepResult :type "HitResult Structure (by ref)"))
  (bind _asbp_third_person_character (cast `/Game/ThirdPerson/Blueprints/BP_ThirdPersonCharacter` OtherActor))
  (`self.EnableInput` (`GameplayStatics.GetPlayerController` 0)))

(event `self.Box.OnComponentEndOverlap`
  (params (OverlappedComponent :type "PrimitiveComponent Object Reference") (OtherActor :type "Actor Object Reference") (OtherComp :type "PrimitiveComponent Object Reference") (OtherBodyIndex :type Integer))
  (cast `/Game/ThirdPerson/Blueprints/BP_ThirdPersonCharacter` OtherActor)
  (`self.DisableInput` (`GameplayStatics.GetPlayerController` 0)))

(fn `UserConstructionScript`)