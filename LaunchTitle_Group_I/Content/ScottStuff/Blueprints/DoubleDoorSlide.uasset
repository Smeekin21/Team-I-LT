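; Double sliding door actor that opens when something overlaps its Box trigger and closes when the overlap ends, with no filter on the overlapping actor.
; A Timeline plays forward on begin overlap and reverses on end overlap.
; Its Slide track lerps the relative locations of DoorHugeTop and DoorHugeBottom between stored current and new Left/Right vectors, without sweeping.
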(event `self.Box.OnComponentBeginOverlap`
  (params (OverlappedComponent :type "PrimitiveComponent Object Reference") (OtherActor :type "Actor Object Reference") (OtherComp :type "PrimitiveComponent Object Reference") (OtherBodyIndex :type Integer) (bFromSweep :type Boolean) (SweepResult :type "HitResult Structure (by ref)"))
  (bind (_direction _slide) (`Timeline|Timeline` :!label _label)
    (:`Update`
      (`SceneComponent.K2_SetRelativeLocation` (`self.door_huge_top`) (`KismetMathLibrary.VLerp` (`self.CurrentLeft`) (`self.NewLeft`) _slide) false false)
      (`SceneComponent.K2_SetRelativeLocation` (`self.door_huge_bottom`) (`KismetMathLibrary.VLerp` (`self.Current Right`) (`self.NewRight`) _slide) false false))))

(event `self.Box.OnComponentEndOverlap`
  (params (OverlappedComponent :type "PrimitiveComponent Object Reference") (OtherActor :type "Actor Object Reference") (OtherComp :type "PrimitiveComponent Object Reference") (OtherBodyIndex :type Integer))
  (goto _label :!via `Reverse`))

(fn `UserConstructionScript`)