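; Turret actor that continuously fires bullets from two spawn points while the player character reference is valid.
; BeginPlay caches the player's BP_ThirdPersonCharacter, which Tick only checks for validity, with no aiming or range test.
; A Delay on Tick throttles the fire rate, then spawns a Bullet_BP at each spawn point with an impulse along the skeletal mesh's right vector.
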(event `self.ReceiveBeginPlay`
  ;[0 0.2243 0.3229] Cast To Player Character Whenever Game Begins
  (bind _asbp_third_person_character (cast `/Game/ThirdPerson/Blueprints/BP_ThirdPersonCharacter` (`GameplayStatics.GetPlayerCharacter` 0)))
  (set `self.As BP Third Person Character` _asbp_third_person_character))

(event `self.ReceiveTick`
  (params (DeltaSeconds :type "Float (single-precision)"))
  (`/Engine/EditorBlueprintResources/StandardMacros.IsValid` (`self.As BP Third Person Character`)
    (:`Is Valid`
      ;[0 0.2159 0.2302] Spawns Bullet 1
      (`KismetSystemLibrary.Delay` 0.3)
      (`|SpawnActorFromClass` "/Game/ThirdPerson/Blueprints/Turrets/Bullet_BP.Bullet_BP_C" (`SceneComponent.K2_GetComponentToWorld` (`self.BulletSpawn1`)) "AdjustIfPossibleButAlwaysSpawn" "MultiplyWithRoot" null (* (`SceneComponent.GetRightVector` (`self.SK_TurretMesh`)) 14000) null)
      ;[0 0.1876 0.201] Spawns Bullet 2
      (`|SpawnActorFromClass` "/Game/ThirdPerson/Blueprints/Turrets/Bullet_BP.Bullet_BP_C" (`SceneComponent.K2_GetComponentToWorld` (`self.BulletSpawn2`)) "Undefined" "MultiplyWithRoot" null (* (`SceneComponent.GetRightVector` (`self.SK_TurretMesh`)) 14000) null))))

(fn `UserConstructionScript`)